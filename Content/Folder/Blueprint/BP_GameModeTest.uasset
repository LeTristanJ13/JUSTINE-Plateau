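; Game mode for a turn-based dice board game, holding player state in BP_GameInstance so it survives returning from another game.
; BeginPlay shows the player-count widget or resumes directly; StartGame spawns pawns on saved cells, applies pending score on return, and spawns the dice.
; RollADice moves the current pawn, triggering the cell's action, then alternates between players 0 and 1, or opens the end map at the last cell.
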(event Custom|StartGame
  (params (NumberPlayers :type Integer))
  (bind _as_bp_game_instance (Variables|Default|GetAs%20BP%20Game%20Instance))
  (bind _as_bp_game_instance_2 (Variables|Default|GetAs%20BP%20Game%20Instance))
  (bind _as_bp_game_instance_3 (Variables|Default|GetAs%20BP%20Game%20Instance))
  ;[1 1 1] Set le nombre de joueurs
  (Variables|Default|SetNumberPlayer NumberPlayers)
  (Variables|/Game/Folder/Blueprint/BP_GameInstance.BP_GameInstance_C|SetNumberOfPlayer (Variables|Default|GetAs%20BP%20Game%20Instance) NumberPlayers)
  (Utilities|FlowControl|Delay 0.2)
  ;[1 1 1] Pour chaque joueurs, récupère sa case, la position de cette case, fais spawn un pion sur cette case, intègre le pion dans la dataStructure S_PlayerData, Spawn le des
  (for _index (range 0 (Variables|Default|GetNumberPlayer))
    (Variables|/Game/Folder/Blueprint/BP_GameInstance.BP_GameInstance_C|SetPlayerTurn (Variables|Default|GetAs%20BP%20Game%20Instance) _index)
    (bind _playercellnumber (Default|GetPlayerCellNumberbyId (Variables|Default|GetAs%20BP%20Game%20Instance) _index))
    (bind _position (Default|GetCellPositionbyNumber (Variables|Default|GetBoardRef) _playercellnumber))
    (bind _returnvalue (Game|SpawnActorfromClass "/Game/Folder/Blueprint/BP_PlayerPion.BP_PlayerPion_C" (Math|Transform|MakeTransform _position "0, 0, 0" "1.000000,1.000000,1.000000") "Undefined" "MultiplyWithRoot" 0 0))
    (Default|SetPlayerPionbyId _as_bp_game_instance _index _returnvalue)
    (if (Variables|/Game/Folder/Blueprint/BP_GameInstance.BP_GameInstance_C|GetIsReturningOfOtherGame _as_bp_game_instance)
      (bind _score (Default|GetPlayerScorebyId _as_bp_game_instance_2 (Variables|/Game/Folder/Blueprint/BP_GameInstance.BP_GameInstance_C|GetPlayerTurn _as_bp_game_instance_2)))
      (Default|SetPlayerScorebyId _as_bp_game_instance_2 (Variables|/Game/Folder/Blueprint/BP_GameInstance.BP_GameInstance_C|GetPlayerTurn _as_bp_game_instance_2) (+ (Variables|/Game/Folder/Blueprint/BP_GameInstance.BP_GameInstance_C|GetScoreTemp _as_bp_game_instance_2) _score))
      (else
        (CallFunction|MovePion _index))))
  (bind _returnvalue_2 (Game|SpawnActorfromClass "/Game/Folder/Blueprint/BP_Des.BP_Des_C" (Math|Transform|MakeTransform "0, 0, 0") "Undefined" "MultiplyWithRoot" 0 0))
  (Variables|Default|SetDice _returnvalue_2)
  (bind _player (Default|GetPlayerbyPlayerTurn _as_bp_game_instance_3 (Variables|/Game/Folder/Blueprint/BP_GameInstance.BP_GameInstance_C|GetPlayerTurn _as_bp_game_instance_3)))
  (Variables|/Game/Folder/Blueprint/Widget/W_Des.W_Des_C|SetPlayer (Variables|/Game/Folder/Blueprint/BP_Des.BP_Des_C|GetW_des _returnvalue_2) _player)
  (Variables|/Game/Folder/Blueprint/BP_GameInstance.BP_GameInstance_C|SetIsReturningOfOtherGame _as_bp_game_instance_3 false)
  (Variables|/Game/Folder/Blueprint/BP_GameInstance.BP_GameInstance_C|SetScoreTemp _as_bp_game_instance_3 0))

(event EventBeginPlay
  ;[1 1 1] Spawn le widget pour choisir nombre joueurs
  (bind _asbp_game_instance (Utilities|Casting|CastToBP_GameInstance (Game|GetGameInstance)))
  (bind _output_get (Variables|Default|SetAs%20BP%20Game%20Instance _asbp_game_instance))
  (if (Variables|/Game/Folder/Blueprint/BP_GameInstance.BP_GameInstance_C|GetIsReturningOfOtherGame _output_get)
    (CallFunction|StartGame (Variables|/Game/Folder/Blueprint/BP_GameInstance.BP_GameInstance_C|GetNumberOfPlayer _output_get))
    (else
      (bind _returnvalue (UserInterface|CreateWidget "/Game/Folder/Blueprint/Widget/W_ChooseNumberPlayer.W_ChooseNumberPlayer_C"))
      (UserInterface|Viewport|AddtoViewport _returnvalue 0))))

(fn ConstructionScript)

(fn RollADice
  (bind _dice (Variables|Default|GetDice))
  (bind _as_bp_game_instance (Variables|Default|GetAs%20BP%20Game%20Instance))
  (bind _playerturn (Variables|/Game/Folder/Blueprint/BP_GameInstance.BP_GameInstance_C|GetPlayerTurn _as_bp_game_instance))
  (bind _w_des (Variables|/Game/Folder/Blueprint/BP_Des.BP_Des_C|GetW_des _dice))
  (Default|RollDice _dice)
  (bind _player (Default|GetPlayerbyPlayerTurn _as_bp_game_instance _playerturn))
  (Variables|/Game/Folder/Blueprint/Widget/W_Des.W_Des_C|SetPlayer _w_des _player)
  (Variables|/Game/Folder/Blueprint/Widget/W_Des.W_Des_C|SetScore _w_des (.Score (Utilities|Struct|BreakS_PlayerData _player)))
  ;[1 1 1] Récupère la case du joueur
  (bind _playercellnumber (Default|GetPlayerCellNumberbyId (Variables|Default|GetAs%20BP%20Game%20Instance) _playerturn))
  ;[1 1 1] Vérifie AVANT de bouger le pion l'index de la case
  (bind _itslastcell (CallFunction|CheckifItstheEnd (+ _playercellnumber (Variables|/Game/Folder/Blueprint/BP_Des.BP_Des_C|GetResultat _dice))))
  (bind _lastcellindex (Utilities|EndOftheGame _itslastcell)
    (:GameContinue
      (CallFunction|MovePion (Variables|/Game/Folder/Blueprint/BP_GameInstance.BP_GameInstance_C|GetPlayerTurn (Variables|Default|GetAs%20BP%20Game%20Instance)) (+ _playercellnumber (Variables|/Game/Folder/Blueprint/BP_Des.BP_Des_C|GetResultat _dice)))
      (CallFunction|ChangeTurn))
    (:EndOfTheGame
      (CallFunction|MovePion (Variables|/Game/Folder/Blueprint/BP_GameInstance.BP_GameInstance_C|GetPlayerTurn (Variables|Default|GetAs%20BP%20Game%20Instance)) _lastcellindex)
      (Viewport|RemoveAllWidgets)
      (Game|OpenLevel(byObjectReference) "/Game/MapFin.MapFin"))))

(fn CheckifItstheEnd
  (params (CellIndex :type Integer))
  ;[1 1 1] Si l'index de la case est supérieure ou égale à la taille de la liste des cases -1, met boolean sur true
  (return (>= CellIndex (- (Utilities|Array|Length (Variables|/Game/Folder/Blueprint/BP_Board.BP_Board_C|GetCellList (Variables|Default|GetBoardRef))) 1))))

(fn ChangeTurn
  ;[1 1 1] Si le nombre de player est supérieur à 0, lance le tour par tour
  (if (not (== (Variables|Default|GetNumberPlayer) 0))
    ;[1 1 1] Si c'est le tour du joueur "0", ++. Si c'est le tour du joueur 1, --.
    (if (== (Variables|/Game/Folder/Blueprint/BP_GameInstance.BP_GameInstance_C|GetPlayerTurn (Variables|Default|GetAs%20BP%20Game%20Instance)) 0)
      (Math|Integer|IncrementInt (Variables|/Game/Folder/Blueprint/BP_GameInstance.BP_GameInstance_C|GetPlayerTurn (Variables|Default|GetAs%20BP%20Game%20Instance))
        (:%20%20
          _))
      (else
        (Math|Integer|DecrementInt (Variables|/Game/Folder/Blueprint/BP_GameInstance.BP_GameInstance_C|GetPlayerTurn (Variables|Default|GetAs%20BP%20Game%20Instance))
          (:%20%20
            _))))
    (Development|PrintString "Changement de joueur ")))

(fn MovePion
  (params (PlayerId :type Integer) (CellNumber :type Integer))
  (bind _boardref (Variables|Default|GetBoardRef))
  (bind _as_bp_game_instance (Variables|Default|GetAs%20BP%20Game%20Instance))
  (Default|SetPlayerCellNumberbyId (Variables|Default|GetAs%20BP%20Game%20Instance) PlayerId CellNumber)
  (bind _position (Default|GetCellPositionbyNumber _boardref CellNumber))
  (Default|MovetoNewCell (.PionRef (Utilities|Struct|BreakS_PlayerData (Utilities|Array|Get(acopy) (Variables|/Game/Folder/Blueprint/BP_GameInstance.BP_GameInstance_C|GetPlayerList _as_bp_game_instance) (Variables|/Game/Folder/Blueprint/BP_GameInstance.BP_GameInstance_C|GetPlayerTurn _as_bp_game_instance)))) _position)
  (bind _player (Default|GetPlayerbyPlayerTurn (Variables|Default|GetAs%20BP%20Game%20Instance) PlayerId))
  (Default|Action (Utilities|Array|Get(acopy) (Variables|/Game/Folder/Blueprint/BP_Board.BP_Board_C|GetCellList _boardref) CellNumber) _player))