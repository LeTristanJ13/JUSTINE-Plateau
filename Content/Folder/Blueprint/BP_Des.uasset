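; BP_Des is a dice-rolling actor that displays its result through an on-screen widget.
; On BeginPlay it creates the W_Des widget, adds it to the viewport and binds its RollBtn click to the Roll event.
; Roll calls RollDice, which sums DiceNumber random rolls from 1 to DiceType and writes the running total to the ShowResultat text, then prints a debug string.
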(event Custom|Roll
  ;[1 1 1] Roll le dès quand je clique sur le bouton
  (CallFunction|RollDice)
  (Development|PrintString "Hello"))

(event EventBeginPlay
  (bind _returnvalue (UserInterface|CreateWidget "/Game/Folder/Blueprint/Widget/W_Des.W_Des_C"))
  (Variables|Default|SetW_des _returnvalue)
  (UserInterface|Viewport|AddtoViewport _returnvalue 0)
  (EventDispatchers|BindEventtoOnClicked (Variables|/Game/Folder/Blueprint/Widget/W_Des.W_Des_C|GetRollBtn (Variables|Default|GetW_des)) (delegate Custom|Roll)))

(event Collision|EventActorBeginOverlap
  (params (OtherActor :type Actor%20Object%20Reference)))

(event EventTick
  (params (DeltaSeconds :type Float%20%28single-precision%29)))

(fn ConstructionScript)

(fn RollDice
  (Variables|Default|SetResultat 0)
  (for _index (range 1 (Variables|Default|GetDiceNumber))
    (Variables|Default|SetResultat (+ (Variables|Default|GetResultat) (Math|Random|RandomIntegerinRange 1 (Variables|Default|GetDiceType))))
    (Variables|/Script/UMG.TextBlock|SetText (Variables|/Game/Folder/Blueprint/Widget/W_Des.W_Des_C|GetShowResultat (Variables|Default|GetW_des)) (Utilities|Text|ToText(Integer) (Variables|Default|GetResultat)))))