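; Game mode for the Memory card minigame, which creates the score widget and resolves card clicks.
; It holds the first clicked card and compares colors with the next: matches are destroyed and score a point, mismatches are both toggled.
; When the card list empties, it stores the score plus a bonus and a return flag in BP_GameInstance, then opens MapTest.
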(event EventBeginPlay
  (bind _asbp_game_instance (Utilities|Casting|CastToBP_GameInstance (Game|GetGameInstance)))
  (Variables|Default|SetAs%20BP%20Game%20Instance _asbp_game_instance)
  (bind _returnvalue (UserInterface|CreateWidget "/Game/Folder/Blueprint/MiniJeu/Memory/W_Memory.W_Memory_C"))
  (bind _output_get (Variables|Default|SetMemoryWB _returnvalue))
  (UserInterface|Viewport|AddtoViewport _output_get 0))

(event EventTick
  (params (DeltaSeconds :type Float%20%28single-precision%29)))

(fn ConstructionScript)

(fn OnCardClicked
  (params (CardRef :type BP%20Card%20Object%20Reference))
  (if (Utilities|IsValid (Variables|Default|GetPreCard))
    (if (Utilities|Enum|Equal(Enum) (Variables|/Game/Folder/Blueprint/MiniJeu/Memory/BP_Card.BP_Card_C|GetColor CardRef) (Variables|/Game/Folder/Blueprint/MiniJeu/Memory/BP_Card.BP_Card_C|GetColor (Variables|Default|GetPreCard)))
      (if (not (== CardRef (Variables|Default|GetPreCard)))
        (bind _result (Math|Integer|IncrementInt (Variables|Default|GetScore))
          (:%20%20
            (Variables|Default|SetScore _result)
            (Utilities|Array|RemoveItem (Variables|Default|GetCardList) (Variables|Default|GetPreCard))
            (Actor|DestroyActor (Variables|Default|GetPreCard))
            (Variables|Default|SetPreCard 0)
            (Utilities|Array|RemoveItem (Variables|Default|GetCardList) CardRef)
            (Actor|DestroyActor CardRef)
            (Variables|/Script/UMG.TextBlock|SetText (Variables|/Game/Folder/Blueprint/MiniJeu/Memory/W_Memory.W_Memory_C|GetScore (Variables|Default|GetMemoryWB)) (Utilities|Text|ToText(Integer) (Variables|Default|GetScore)))
            (CallFunction|CheckiftheGameEnd)))
        (else
          (Variables|Default|SetPreCard 0)))
      (else
        (Default|ToggleCard (Variables|Default|GetPreCard))
        (Default|ToggleCard CardRef)
        (Variables|Default|SetPreCard 0)))
    (else
      (Variables|Default|SetPreCard CardRef))))

(fn CheckiftheGameEnd
  (bind _as_bp_game_instance (Variables|Default|GetAs%20BP%20Game%20Instance))
  (if (== (Utilities|Array|Length (Variables|Default|GetCardList)) 0)
    (Variables|/Game/Folder/Blueprint/BP_GameInstance.BP_GameInstance_C|SetIsReturningOfOtherGame _as_bp_game_instance true)
    (Variables|/Game/Folder/Blueprint/BP_GameInstance.BP_GameInstance_C|SetScoreTemp _as_bp_game_instance (+ (Variables|Default|GetScore) 200))
    (Game|OpenLevel(byObjectReference) "/Game/MapTest.MapTest")))