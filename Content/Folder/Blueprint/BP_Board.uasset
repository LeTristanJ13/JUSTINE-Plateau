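; BP_Board is the game board actor that maps cell indices to world positions for players.
; On BeginPlay it caches BP_GameModeTest and registers itself as that game mode's BoardRef.
; GetCellPositionByNumber looks up a cell in CellList and, when NumberPlayer is above zero, returns its Spawn1 or Spawn2 location based on the game instance's PlayerTurn.
; Otherwise it returns the cell actor's own location.
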(event EventBeginPlay
  (bind _asbp_game_mode_test (Utilities|Casting|CastToBP_GameModeTest (Game|GetGameMode)))
  (Variables|Default|SetAs%20BP%20Game%20Mode%20Test _asbp_game_mode_test)
  (Variables|/Game/Folder/Blueprint/BP_GameModeTest.BP_GameModeTest_C|SetBoardRef _asbp_game_mode_test self))

(event Collision|EventActorBeginOverlap
  (params (OtherActor :type Actor%20Object%20Reference)))

(event EventTick
  (params (DeltaSeconds :type Float%20%28single-precision%29)))

(fn ConstructionScript)

(fn GetCellPositionbyNumber
  (params (CellIndex :type Integer))
  (bind _celllist (Variables|Default|GetCellList))
  (bind _output (Utilities|Array|Get(acopy) _celllist CellIndex))
  (if (> (Variables|/Game/Folder/Blueprint/BP_GameModeTest.BP_GameModeTest_C|GetNumberPlayer (Variables|Default|GetAs%20BP%20Game%20Mode%20Test)) 0)
    (if (== (Variables|/Game/Folder/Blueprint/BP_GameInstance.BP_GameInstance_C|GetPlayerTurn (Variables|/Game/Folder/Blueprint/BP_GameModeTest.BP_GameModeTest_C|GetAs%20BP%20Game%20Instance (Variables|Default|GetAs%20BP%20Game%20Mode%20Test))) 0)
      (return (Transformation|GetWorldLocation (Variables|/Game/Folder/Blueprint/BP_Cell.BP_Cell_C|GetSpawn1 _output)))
      (else
        (return (Transformation|GetWorldLocation (Variables|/Game/Folder/Blueprint/BP_Cell.BP_Cell_C|GetSpawn2 _output)))))
    (else
      (return (Transformation|GetActorLocation _output)))))