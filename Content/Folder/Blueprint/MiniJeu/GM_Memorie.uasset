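; Game mode, judging by its GM_ prefix, for a memory card mini-game, holding the pair-matching rules and score.
; OnCardClicked stores the first card as PreCard, then compares the next card's Color against it.
; A match increments Score and destroys both cards; a mismatch toggles both but leaves PreCard set.
; ReturnCard and the event graph are empty stubs, and CardList is unused.
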(event EventBeginPlay)

(event EventTick
  (params (DeltaSeconds :type Float%20%28single-precision%29)))

(fn ConstructionScript)

(fn ReturnCard)

(fn OnCardClicked
  (params (CardRef :type BP%20Card%20Object%20Reference))
  (if (Utilities|IsValid (Variables|Default|GetPreCard))
    (if (Utilities|Enum|Equal(Enum) (Variables|/Game/Folder/Blueprint/MiniJeu/BP_Card.BP_Card_C|GetColor CardRef) (Variables|/Game/Folder/Blueprint/MiniJeu/BP_Card.BP_Card_C|GetColor (Variables|Default|GetPreCard)))
      (bind _result (Math|Integer|IncrementInt (Variables|Default|GetScore))
        (:%20%20
          (Variables|Default|SetScore _result)
          (Actor|DestroyActor (Variables|Default|GetPreCard))
          (Variables|Default|SetPreCard 0)
          (Actor|DestroyActor CardRef)
          (Development|PrintString "Hello")))
      (else
        (Default|ToggleCard (Variables|Default|GetPreCard))
        (Default|ToggleCard CardRef)))
    (else
      (Variables|Default|SetPreCard CardRef))))