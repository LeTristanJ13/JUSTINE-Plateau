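; BP_CellScorePlus is a cell Blueprint that adds points to a player's score when its Action runs.
; Its Action override calls the parent, then adds ValeurScore to the player's current Score and writes the total to the game instance, reached through the game mode, by PlayerNumber.
; A yellow debug print follows, with the event graph holding only disabled default nodes.
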(event EventBeginPlay
  (|CallParentFunction) ; This node is disabled and will not be called.\nDrag off pins to build functionality.
)

(event Collision|EventActorBeginOverlap
  (params (OtherActor :type Actor%20Object%20Reference))
  (|CallParentFunction OtherActor) ; This node is disabled and will not be called.\nDrag off pins to build functionality.
)

(event EventTick
  (params (DeltaSeconds :type Float%20%28single-precision%29))
  (|CallParentFunction DeltaSeconds) ; This node is disabled and will not be called.\nDrag off pins to build functionality.
)

(fn ConstructionScript
  (|CallParentFunction))

(fn Action
  (params (Player :type S%20Player%20Data%20Structure))
  (bind (_playernumber _score) (Utilities|Struct|BreakS_PlayerData Player))
  (|CallParentFunction "")
  (Default|SetPlayerScorebyId (Variables|/Game/Folder/Blueprint/BP_GameModeTest.BP_GameModeTest_C|GetAs%20BP%20Game%20Instance (Variables|Default|GetAs%20BP%20Game%20Mode%20Test)) _playernumber (+ _score (LocalVariables|GetValeurScore)))
  (Development|PrintString "Hello" true true "(R=1.000000,G=0.932230,B=0.000000,A=1.000000)" 5.0))