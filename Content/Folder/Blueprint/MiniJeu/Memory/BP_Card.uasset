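; Clickable card actor for the Memory mini-game, with a back-face (Verso) material chosen from its Color value.
; It registers itself in GM_Memorie's CardList on BeginPlay, and a click flips it after a short delay, then reports it through OnCardClicked.
; ToggleCard snaps the root roll between face states and inverts IsClickable, which the click event never checks.
; The construction script and ChangeCardColor share identical color-to-material logic.
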(event EventBeginPlay
  (bind _asgm_memorie (Utilities|Casting|CastToGM_Memorie (Game|GetGameMode)))
  (bind _output_get (Variables|Default|SetAs%20GM%20Memorie _asgm_memorie))
  (Utilities|Array|AddUnique (Variables|/Game/Folder/Blueprint/MiniJeu/Memory/GM_Memorie.GM_Memorie_C|GetCardList _output_get) self))

(event Collision|EventActorBeginOverlap
  (params (OtherActor :type Actor%20Object%20Reference)))

(event EventTick
  (params (DeltaSeconds :type Float%20%28single-precision%29)))

(event MouseInput|EventActorOnClicked
  (params (ButtonPressed :type Key%20Structure :default "None"))
  (Utilities|FlowControl|Delay 0.3)
  (CallFunction|ToggleCard)
  (Utilities|FlowControl|Delay 0.2)
  (Default|OnCardClicked (Variables|Default|GetAs%20GM%20Memorie) self))

(fn ConstructionScript
  (switch Utilities|FlowControl|Switch|SwitchonE_Color (Variables|Default|GetColor)
    (:NewEnumerator0
      (Rendering|Material|SetMaterial (Variables|Default|GetVerso) 0 "/Game/Folder/Material/MI_GoodaCTION.MI_GoodaCTION"))
    (:NewEnumerator1
      (Rendering|Material|SetMaterial (Variables|Default|GetVerso) 0 "/Game/Folder/Material/MI_BadAction.MI_BadAction"))
    (:NewEnumerator2
      (Rendering|Material|SetMaterial (Variables|Default|GetVerso) 0 "/Game/Folder/Material/MI_Color.MI_Color"))
    (:NewEnumerator3
      (Rendering|Material|SetMaterial (Variables|Default|GetVerso) 0 "/Game/Folder/Material/MI_CaseAction.MI_CaseAction"))))

(fn ChangeCardColor
  (switch Utilities|FlowControl|Switch|SwitchonE_Color (Variables|Default|GetColor)
    (:NewEnumerator0
      (Rendering|Material|SetMaterial (Variables|Default|GetVerso) 0 "/Game/Folder/Material/MI_GoodaCTION.MI_GoodaCTION"))
    (:NewEnumerator1
      (Rendering|Material|SetMaterial (Variables|Default|GetVerso) 0 "/Game/Folder/Material/MI_BadAction.MI_BadAction"))
    (:NewEnumerator2
      (Rendering|Material|SetMaterial (Variables|Default|GetVerso) 0 "/Game/Folder/Material/MI_Color.MI_Color"))
    (:NewEnumerator3
      (Rendering|Material|SetMaterial (Variables|Default|GetVerso) 0 "/Game/Folder/Material/MI_CaseAction.MI_CaseAction"))))

(fn ToggleCard
  (Variables|Default|SetisClickable (not (Variables|Default|GetisClickable)))
  (if (== (.roll (.rotation (Transformation|GetWorldTransform (Variables|Default|GetDefaultSceneRoot)))) 0.0)
    (Transformation|SetRelativeRotation (Variables|Default|GetDefaultSceneRoot) (Math|Rotator|MakeRotator 1.8e+02 0.0 0.0) false false)
    (Development|PrintString "rotate")
    (else
      (Transformation|SetRelativeRotation (Variables|Default|GetDefaultSceneRoot) (Math|Rotator|MakeRotator 0.0 0.0 0.0) false false))))