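; BP_CellMiniJeu is a child Blueprint, named as a mini-game cell, that shows an explanation screen when its action runs for a player.
; Its Action override calls the parent, removes all widgets, then creates W_Explication and adds it to the viewport.
; The event graph holds only disabled default events, and the construction script just calls its parent.
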(event EventBeginPlay
  (|CallParentFunction) ; This node is disabled and will not be called.\nDrag off pins to build functionality.
)

(event Collision|EventActorBeginOverlap
  (params (OtherActor :type Actor%20Object%20Reference))
  (|CallParentFunction OtherActor) ; This node is disabled and will not be called.\nDrag off pins to build functionality.
)

(event EventTick
  (params (DeltaSeconds :type Float%20%28single-precision%29))
  (|CallParentFunction DeltaSeconds) ; This node is disabled and will not be called.\nDrag off pins to build functionality.
)

(fn ConstructionScript
  (|CallParentFunction))

(fn Action
  (params (Player :type S%20Player%20Data%20Structure))
  (|CallParentFunction Player)
  (Viewport|RemoveAllWidgets)
  (bind _returnvalue (UserInterface|CreateWidget "/Game/Folder/Blueprint/Widget/W_Explication.W_Explication_C"))
  (UserInterface|Viewport|AddtoViewport _returnvalue 0))