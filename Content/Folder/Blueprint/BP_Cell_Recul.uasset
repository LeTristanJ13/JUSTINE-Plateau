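; Board cell Blueprint that sends a player's pawn backward when its Action runs.
; The Action override calls the parent, then asks BPGameModeTest's MovePion to move that player to their current cell number minus ValeurDeplacement.
; It prints a red French debug message saying "I move back 2", with the distance hardcoded in the text rather than read from the variable.
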(event EventBeginPlay
  (|CallParentFunction) ; This node is disabled and will not be called.\nDrag off pins to build functionality.
)

(event Collision|EventActorBeginOverlap
  (params (OtherActor :type Actor%20Object%20Reference))
  (|CallParentFunction OtherActor) ; This node is disabled and will not be called.\nDrag off pins to build functionality.
)

(event EventTick
  (params (DeltaSeconds :type Float%20%28single-precision%29))
  (|CallParentFunction DeltaSeconds) ; This node is disabled and will not be called.\nDrag off pins to build functionality.
)

(fn ConstructionScript
  (|CallParentFunction))

(fn Action
  (params (Player :type S%20Player%20Data%20Structure))
  (bind (_playernumber _score _cellnumber) (Utilities|Struct|BreakS_PlayerData Player))
  (|CallParentFunction "")
  (Default|MovePion (Variables|Default|GetAs%20BP%20Game%20Mode%20Test) _playernumber (- _cellnumber (LocalVariables|GetValeurDeplacement)))
  (Development|PrintString "Je recule de 2" true true "(R=1.000000,G=0.000000,B=0.083156,A=1.000000)" 6.0))