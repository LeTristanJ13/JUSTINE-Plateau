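; Game mode for the Collectable mini-game that shows elapsed time and ends the session at the two-minute mark.
; On BeginPlay it creates the WB_Collectable HUD widget and caches the BP_GameInstance.
; Each OnAddSecond event refreshes the minute and second text; when Minute reaches two, it flags the game instance as returning from another game and opens MapTest.
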(event EventBeginPlay
  (bind _returnvalue (UserInterface|CreateWidget "/Game/Folder/Blueprint/MiniJeu/Collectable/WB_Collectable.WB_Collectable_C"))
  (UserInterface|Viewport|AddtoViewport _returnvalue 0)
  (Variables|Default|SetW_Collectable _returnvalue)
  (bind _asbp_game_instance (Utilities|Casting|CastToBP_GameInstance (Game|GetGameInstance)))
  (Variables|Default|SetAs%20BP%20Game%20Instance _asbp_game_instance))

(event EventOnAddSecond
  (bind _minute (Variables|Default|GetMinute))
  (bind _w_collectable (Variables|Default|GetW_Collectable))
  (Variables|/Script/UMG.TextBlock|SetText (Variables|/Game/Folder/Blueprint/MiniJeu/Collectable/WB_Collectable.WB_Collectable_C|GetMinute _w_collectable) (Utilities|Text|ToText(Integer) _minute))
  (Variables|/Script/UMG.TextBlock|SetText (Variables|/Game/Folder/Blueprint/MiniJeu/Collectable/WB_Collectable.WB_Collectable_C|GetSeconde _w_collectable) (Utilities|Text|ToText(Integer) (Variables|Default|GetSeconde)))
  (if (== _minute 2)
    (Variables|/Game/Folder/Blueprint/BP_GameInstance.BP_GameInstance_C|SetIsReturningOfOtherGame (Variables|Default|GetAs%20BP%20Game%20Instance) true)
    (Game|OpenLevel(byObjectReference) "/Game/MapTest.MapTest")))

(fn ConstructionScript)