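; BP_Cell is a cell actor that provides per-player spawn positions and an Action hook, likely a base for board cell types.
; On BeginPlay it casts the game mode to BP_GameModeTest and caches the reference.
; GetSocketPosByPlayerID reads the world location of Spawn1 for player 0 or Spawn2 otherwise, though only the player 0 branch returns it.
; Action takes a player and is empty here.
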(event EventBeginPlay
  (bind _asbp_game_mode_test (Utilities|Casting|CastToBP_GameModeTest (Game|GetGameMode)))
  (Variables|Default|SetAs%20BP%20Game%20Mode%20Test _asbp_game_mode_test))

(event Collision|EventActorBeginOverlap
  (params (OtherActor :type Actor%20Object%20Reference)))

(event EventTick
  (params (DeltaSeconds :type Float%20%28single-precision%29)))

(fn ConstructionScript)

(fn GetSocketPosbyPlayerID
  (params (PlayerId :type Integer))
  (if (== PlayerId 0)
    (LocalVariables|SetTempSocketPos (Transformation|GetWorldLocation (Variables|Default|GetSpawn1)))
    (return (LocalVariables|GetTempSocketPos))
    (else
      (LocalVariables|SetTempSocketPos (Transformation|GetWorldLocation (Variables|Default|GetSpawn2))))))

(fn Action
  (params (Player :type S%20Player%20Data%20Structure)))