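; Game mode for a board game that spawns a pawn on the starting cell when play begins.
; After a short delay, BeginPlay caches the custom game instance, asks the board reference for the first cell's position and spawns a single BP_Pion there.
; SendInformationsGI, not called in this graph, loops over an array to number players by index and reset their cell to the start.
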(event EventBeginPlay
  (Utilities|FlowControl|Delay 0.2)
  (bind _asbp_game_instance (Utilities|Casting|CastToBP_GameInstance (Game|GetGameInstance)))
  (Variables|Default|SetAs%20BP%20Game%20Instance _asbp_game_instance)
  (bind _newparam (Default|GetCellPositionbyNumber (Variables|Default|GetBoardRef)))
  (Game|SpawnActorfromClass "/Game/Folder/Blueprint/BP_Pion.BP_Pion_C" (Math|Transform|MakeTransform _newparam "0, 0, 0" "1.000000,1.000000,1.000000") "Undefined" "MultiplyWithRoot" 0 0))

(event EventTick
  (params (DeltaSeconds :type Float%20%28single-precision%29)))

(fn ConstructionScript)

(fn SendInformationsGI
  (for (_array_element _array_index) 0
    (|SetBy-RefVar (.PlayerNumber (Utilities|Struct|BreakS_PlayerData _array_element)) _array_index)
    (|SetBy-RefVar (.CellNumber (Utilities|Struct|BreakS_PlayerData _array_element)))))